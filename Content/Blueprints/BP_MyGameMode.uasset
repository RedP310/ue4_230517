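; Game mode Blueprint that puts the player UI on screen and keeps the total score.
; BeginPlay creates the PlayerUI widget and adds it to the viewport, and AddScore increments TotalScore by one.
; A disconnected chain that would set Exploding once PassedLights equals the number of BP_Light actors never runs, and Tick is empty.
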(event `self.ReceiveBeginPlay`
  (bind _returnvalue (`|CreateWidget` "/Game/UMG/PlayerUI.PlayerUI_C"))
  (`UserWidget.AddToViewport` _returnvalue 0))

(event `self.ReceiveTick`
  (params (DeltaSeconds :type "Float (single-precision)")))

(fn `AddScore`
  (set `self.TotalScore` (+ (`self.TotalScore`) 1)))

(fn `UserConstructionScript`)